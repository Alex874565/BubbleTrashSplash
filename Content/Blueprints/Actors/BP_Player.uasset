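; BP_Player is a Paper2D player that moves along X and Z and plays a pick-up animation.
; BeginPlay adds the Enhanced Input mapping, then shuffles the BP_WasteSpawner actors and spawns BP_Waste at random spawner locations until WasteNo runs out.
; Horizontal input rotates the sprite to face the movement direction.
; Pick-up input only swaps flipbooks, returning to idle after a short delay, with no collection logic.
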(event `self.ReceiveBeginPlay`
  (bind _wasteno (`self.WasteNo`))
  (`EnhancedInputSubsystemInterface.AddMappingContext` (pcsubsystem `EnhancedInputLocalPlayerSubsystem` (`GameplayStatics.GetPlayerController` 0)) "/Game/Blueprints/IMC_Main.IMC_Main" 0 (struct))
  (bind _outactors (`GameplayStatics.GetAllActorsOfClass` "/Game/Blueprints/Actors/BP_WasteSpawner.BP_WasteSpawner_C"))
  (`KismetArrayLibrary.Array_Shuffle` _outactors)
  (for _array_element _outactors
    (if (> _wasteno 0)
      (set `self.WasteNo` (- _wasteno 1))
      (`|SpawnActorFromClass` "/Game/Blueprints/Actors/BP_Waste.BP_Waste_C" (`KismetMathLibrary.MakeTransform` (`self.K2_GetActorLocation` _array_element)) "AdjustIfPossibleButAlwaysSpawn" "MultiplyWithRoot" null null)
      (`KismetSystemLibrary.PrintString` "Hello")
      (else
        (break)))))

(event `EnhancedInput|/Game/Blueprints/IA_Horizontal`
  (params (ActionValue :type "Float (double-precision)") (ElapsedSeconds :type "Float (double-precision)") (TriggeredSeconds :type "Float (double-precision)") (InputAction :type "InputAction Object Reference" :default "/Game/Blueprints/IA_Horizontal.IA_Horizontal"))
  (bind _sprite (`self.Sprite`))
  (:`Triggered`
    (`self.AddMovementInput` (1.0 0.0 0.0) ActionValue)
    (if (> ActionValue 0.0)
      (`SceneComponent.K2_SetWorldRotation` _sprite (struct :`Pitch` -90.0) false false)
      (else
        (`SceneComponent.K2_SetWorldRotation` _sprite (struct :`Pitch` -90.0 :`Yaw` 180.0) false false)))))

(event `EnhancedInput|/Game/Blueprints/IA_Vertical`
  (params (ActionValue :type "Float (double-precision)") (ElapsedSeconds :type "Float (double-precision)") (TriggeredSeconds :type "Float (double-precision)") (InputAction :type "InputAction Object Reference" :default "/Game/Blueprints/IA_Vertical.IA_Vertical"))
  (:`Triggered`
    (`self.AddMovementInput` (0.0 0.0 1.0) ActionValue)))

(event `EnhancedInput|/Game/Blueprints/IA_PickUp`
  (params (ActionValue :type Boolean) (ElapsedSeconds :type "Float (double-precision)") (TriggeredSeconds :type "Float (double-precision)") (InputAction :type "InputAction Object Reference" :default "/Game/Blueprints/IA_PickUp.IA_PickUp"))
  (:`Triggered`
    (`PaperFlipbookComponent.SetFlipbook` (`self.Sprite`) "/Game/SpearFishing_Assets_Pack/Sprites/Diver-32x32/FB_PickUp.FB_PickUp"))
  (:`Completed`
    (`KismetSystemLibrary.Delay` 0.4)
    (`PaperFlipbookComponent.SetFlipbook` (`self.Sprite`) "/Game/SpearFishing_Assets_Pack/Sprites/Diver-32x32/FB_Idle.FB_Idle")))

(event `self.ReceiveActorBeginOverlap`
  (params (OtherActor :type "Actor Object Reference")))

(fn `UserConstructionScript`)