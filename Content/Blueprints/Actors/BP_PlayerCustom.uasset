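; Player character for an underwater Paper2D game about collecting waste before oxygen runs out.
; BeginPlay spawns waste at shuffled BP_WasteSpawner points, which a looping timer reuses for bubbles.
; Enhanced Input drives movement and sphere-trace pickups that earn money; bubbles refill oxygen, with upgrade levels scaling both.
; Empty oxygen or non-bubble overlaps cause death and a saved money penalty, while surfacing opens the end-mission menu.
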(event `self.ReceiveBeginPlay`
  (bind _returnvalue (`GameplayStatics.GetPlayerController` 0))
  (bind _wasteno (`self.WasteNo`))
  (bind _asbp_my_game_instance (cast `/Game/Blueprints/BP_MyGameInstance` (`GameplayStatics.GetGameInstance`)))
  (if (not (`self.PlayingMusic`))
    (`/Game/Blueprints/BP_MyGameInstance.Play Music` _asbp_my_game_instance "/Game/Underwater_Blues__Royalty_Free_Game_Music_.Underwater_Blues__Royalty_Free_Game_Music_"))
  (`WidgetBlueprintLibrary.SetInputMode_GameOnly` _returnvalue)
  (set `self.Oxygen` (+ (`self.MaxOxygen`) (* (`self.OxygenLevel`) 2)))
  (`PaperFlipbookComponent.SetLooping` (`self.PaperFlipbook`) true)
  (`EnhancedInputSubsystemInterface.AddMappingContext` (pcsubsystem `EnhancedInputLocalPlayerSubsystem` _returnvalue) "/Game/Blueprints/IMC_Main.IMC_Main" 0 (struct))
  (set `self.WasteNo` (+ 5 (`self.MoneyLevel`)))
  (bind _outactors (`GameplayStatics.GetAllActorsOfClass` "/Game/Blueprints/Actors/BP_WasteSpawner.BP_WasteSpawner_C"))
  (`KismetArrayLibrary.Array_Shuffle` _outactors)
  (for _array_element _outactors
    (if (> _wasteno 0)
      (set `self.WasteNo` (- _wasteno 1))
      (`|SpawnActorFromClass` "/Game/Blueprints/Actors/BP_Waste.BP_Waste_C" (`KismetMathLibrary.MakeTransform` (+ (`self.K2_GetActorLocation` _array_element) (0.0 0.0 2.0))) "AdjustIfPossibleButAlwaysSpawn" "MultiplyWithRoot" null null)
      (`KismetSystemLibrary.K2_SetTimer` null "SpawnBubble" 2.0 true)
      (bind _returnvalue_2 (`|CreateWidget` "/Game/Widgets/W_HUD.W_HUD_C"))
      (`UserWidget.AddToViewport` _returnvalue_2 0)
      (else
        (break)))))

(event `self.ReceiveTick`
  (params (DeltaSeconds :type "Float (single-precision)"))
  (bind (_returnvalue_x _returnvalue_y _returnvalue_z) (`KismetMathLibrary.BreakVector` (`self.K2_GetActorLocation`)))
  (bind _returnvalue (`GameplayStatics.GetPlayerController` 0))
  (bind _returnvalue_2 (`GameplayStatics.GetPlayerController` 0))
  (bind _money (`self.Money`))
  (bind _returnvalue_roll (`KismetMathLibrary.BreakRotator` (`SceneComponent.K2_GetComponentRotation` (`self.PaperFlipbook`))))
  (if (not (`self.Dead`))
    (bind _output_get (set `self.Oxygen` (- (`self.Oxygen`) DeltaSeconds)))
    (if (<= _output_get 0.0)
      (bind _output_get_2 (set `self.Money` (- _money (`KismetMathLibrary.Min` _money (- 30 (`self.MoneyLevel`)))) :!label _label))
      (bind _returnvalue_3 (`GameplayStatics.LoadGameFromSlot` "save"))
      (bind _asbp_save (cast `/Game/Blueprints/BP_Save` _returnvalue_3))
      (set `/Game/Blueprints/BP_Save.Money` _output_get_2 _asbp_save)
      (`GameplayStatics.SaveGameToSlot` _asbp_save "save")
      (set `self.Dead` true)
      (`self.DisableInput` (`GameplayStatics.GetPlayerController` 0))
      (`PaperFlipbookComponent.SetFlipbook` (`self.PaperFlipbook`) "/Game/SpearFishing_Assets_Pack/Sprites/Diver-32x32/FB_Death.FB_Death")
      (`PaperFlipbookComponent.SetLooping` (`self.PaperFlipbook`) false)
      (set `PlayerController.bShowMouseCursor` true _returnvalue)
      (bind _returnvalue_4 (`|CreateWidget` "/Game/Widgets/W_DeathMenu.W_DeathMenu_C"))
      (`UserWidget.AddToViewport` _returnvalue_4 0)
      (`WidgetBlueprintLibrary.SetInputMode_UIOnlyEx` _returnvalue _returnvalue_4)
      (`KismetSystemLibrary.MoveComponentTo` (`self.PaperFlipbook`) (- (`self.K2_GetActorLocation`) (0.0 0.0 16.0)) (`KismetMathLibrary.MakeRotator` 0.0 0.0 (- 180.0 _returnvalue_roll)) false false 4.0)
      (`GameplayStatics.SetGamePaused` true)
      (elif (> _returnvalue_z 12.0)
        (`self.K2_SetActorLocation` (`KismetMathLibrary.MakeVector` _returnvalue_x _returnvalue_y (- _returnvalue_z 10.0)))
        (`GameplayStatics.SetGamePaused` true)
        (set `PlayerController.bShowMouseCursor` true _returnvalue_2)
        (bind _returnvalue_5 (`|CreateWidget` "/Game/Widgets/W_EndMission.W_EndMission_C"))
        (`UserWidget.AddToViewport` _returnvalue_5 0)
        (`WidgetBlueprintLibrary.SetInputMode_UIOnlyEx` _returnvalue_2 _returnvalue_5)))))

(event `EnhancedInput|/Game/Blueprints/IA_Horizontal`
  (params (ActionValue :type "Float (double-precision)") (ElapsedSeconds :type "Float (double-precision)") (TriggeredSeconds :type "Float (double-precision)") (InputAction :type "InputAction Object Reference" :default "/Game/Blueprints/IA_Horizontal.IA_Horizontal"))
  (bind _paperflipbook (`self.PaperFlipbook`))
  (:`Triggered`
    (`self.AddMovementInput` (1.0 0.0 0.0) ActionValue)
    (if (> ActionValue 0.0)
      (`SceneComponent.K2_SetWorldRotation` _paperflipbook (struct :`Pitch` -90.0) false false)
      (else
        (`SceneComponent.K2_SetWorldRotation` _paperflipbook (struct :`Pitch` -90.0 :`Yaw` 180.0) false false)))))

(event `EnhancedInput|/Game/Blueprints/IA_Vertical`
  (params (ActionValue :type "Float (double-precision)") (ElapsedSeconds :type "Float (double-precision)") (TriggeredSeconds :type "Float (double-precision)") (InputAction :type "InputAction Object Reference" :default "/Game/Blueprints/IA_Vertical.IA_Vertical"))
  (:`Triggered`
    (`self.AddMovementInput` (0.0 0.0 1.0) ActionValue)))

(event `EnhancedInput|/Game/Blueprints/IA_PickUp`
  (params (ActionValue :type Boolean) (ElapsedSeconds :type "Float (double-precision)") (TriggeredSeconds :type "Float (double-precision)") (InputAction :type "InputAction Object Reference" :default "/Game/Blueprints/IA_PickUp.IA_PickUp"))
  (bind _paperflipbook (`self.PaperFlipbook`))
  (bind _returnvalue (+ (`self.K2_GetActorLocation`) (0.0 0.0 -1.0)))
  (:`Triggered`
    (`PaperFlipbookComponent.SetFlipbook` _paperflipbook "/Game/SpearFishing_Assets_Pack/Sprites/Diver-32x32/FB_PickUp.FB_PickUp")
    (bind (_outhit _returnvalue_2) (`KismetSystemLibrary.SphereTraceSingle` _returnvalue (+ _returnvalue (0.0 0.0 -2.0)) 6.0 "TraceTypeQuery3"))
    (if _returnvalue_2
      (`self.K2_DestroyActor` (`.HitActor` (`GameplayStatics.BreakHitResult` _outhit)))
      (set `self.CollectedWaste` (+ (`self.CollectedWaste`) 1))
      (set `self.Money` (+ (+ (`self.Money`) 10) (* (`self.MoneyLevel`) 2)))))
  (:`Completed`
    (`KismetSystemLibrary.Delay` 0.4)
    (`PaperFlipbookComponent.SetFlipbook` _paperflipbook "/Game/SpearFishing_Assets_Pack/Sprites/Diver-32x32/FB_Idle.FB_Idle")))

(event `self.ReceiveActorBeginOverlap`
  (params (OtherActor :type "Actor Object Reference"))
  (if (`self.Dead`)
    _
    (elif (`self.ActorHasTag` OtherActor "bubble")
      (set `self.Oxygen` (+ (`self.Oxygen`) (+ (`self.BubbleLevel`) 4)))
      (else
        (goto _label)))))

(event `Key|Escape`
  (params (Key :type "Key Structure"))
  (bind _returnvalue (`GameplayStatics.GetPlayerController` 0))
  (:`Pressed`
    (if (not (`self.Dead`))
      (`GameplayStatics.SetGamePaused` true)
      (set `PlayerController.bShowMouseCursor` true _returnvalue)
      (bind _returnvalue_2 (`|CreateWidget` "/Game/Widgets/W_PauseMenu.W_PauseMenu_C"))
      (`UserWidget.AddToViewport` _returnvalue_2 0)
      (`WidgetBlueprintLibrary.SetInputMode_UIOnlyEx` _returnvalue _returnvalue_2))))

(fn `SpawnBubble`
  (bind _outactors (`GameplayStatics.GetAllActorsOfClass` "/Game/Blueprints/Actors/BP_WasteSpawner.BP_WasteSpawner_C"))
  (`KismetArrayLibrary.Array_Shuffle` _outactors)
  (for (_array_element _array_index) _outactors
    (if (>= _array_index (+ (`self.BubbleLevel`) 1))
      (break)
      (else
        (`|SpawnActorFromClass` "/Game/Blueprints/Actors/BP_Bubble.BP_Bubble_C" (`KismetMathLibrary.MakeTransform` (`self.K2_GetActorLocation` _array_element)) "AlwaysSpawn" "MultiplyWithRoot" null null)))))

(fn `UserConstructionScript`)